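; Player ship Character for an Asteroids game, steered with Enhanced Input: yaw turning, forward-only thrust, and zero ground friction with low braking for a floaty drift.
; Shooting spawns the active projectile class, which EquipWeapon swaps temporarily before a timer restores the laser blast.
; Hitting an asteroid while unshielded costs a life and recenters the ship, then re-shields it or reloads the level when lives run out.
; Also tracks points, creates the HUD, and starts with a timed shield overlay.
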(event `self.ReceiveBeginPlay`
  (bind _charactermovement (`self.CharacterMovement`))
  ;[1 1 1] Initialize input mapping
  (bind _asasteroids_player_controller (cast `AsteroidsPlayerController` (`self.GetController`)))
  (bind _returnvalue (pcsubsystem `EnhancedInputLocalPlayerSubsystem` _asasteroids_player_controller))
  (`/Engine/EditorBlueprintResources/StandardMacros.IsValid` _returnvalue
    (:`Is Valid`
      (`EnhancedInputSubsystemInterface.AddMappingContext` _returnvalue "/Game/Asteroids/Input/IMC_AsteroidsPlayer.IMC_AsteroidsPlayer" 0 (struct))
      ;[1 1 1] Set movement to be floaty
      (set `CharacterMovementComponent.GroundFriction` 0.0 _charactermovement)
      (set `CharacterMovementComponent.BrakingDecelerationWalking` 200.0 _charactermovement)
      (bind _returnvalue_2 (`|CreateWidget` "/Game/Asteroids/UI/W_HUD.W_HUD_C"))
      (`UserWidget.AddToViewport` _returnvalue_2 0)
      (`self.ActivateShield`))))

(event `EnhancedInput|/Game/Asteroids/Input/IA_Move`
  (params (ActionValue :type "Vector2D Structure") (ElapsedSeconds :type "Float (double-precision)") (TriggeredSeconds :type "Float (double-precision)") (InputAction :type "InputAction Object Reference" :default "/Game/Asteroids/Input/IA_Move.IA_Move"))
  (:`Triggered`
    ;[1 1 1] Add rotation and movement to the player from input
    (`SceneComponent.K2_AddRelativeRotation` (`self.CapsuleComponent`) (`KismetMathLibrary.MakeRotator` 0.0 0.0 ActionValue_X) false false)
    (`self.AddMovementInput` (`self.GetActorForwardVector`) (`KismetMathLibrary.FClamp` ActionValue_Y))))

(event `EnhancedInput|/Game/Asteroids/Input/IA_Shoot`
  (params (ActionValue :type Boolean) (ElapsedSeconds :type "Float (double-precision)") (TriggeredSeconds :type "Float (double-precision)") (InputAction :type "InputAction Object Reference" :default "/Game/Asteroids/Input/IA_Shoot.IA_Shoot"))
  (:`Triggered`
    (`|SpawnActorFromClass` (`self.ActiveProjectile`) (`KismetMathLibrary.MakeTransform` (`SceneComponent.K2_GetComponentLocation` (`self.ShootLoc`)) (`self.K2_GetActorRotation`)) "Undefined" "MultiplyWithRoot" null null)))

(event `self.CapsuleComponent.OnComponentHit`
  (params (HitComponent :type "PrimitiveComponent Object Reference") (OtherActor :type "Actor Object Reference") (OtherComp :type "PrimitiveComponent Object Reference") (NormalImpulse :type "Vector Structure") (Hit :type "HitResult Structure (by ref)"))
  (cast `/Game/Asteroids/Combat/BP_Asteroid` OtherActor)
  (if (not (`self.bShielded`))
    (`/Engine/EditorBlueprintResources/StandardMacros.DecrementInt` (`self.Lives`)
      (:`  `
        (`self.K2_SetActorLocation` (0.0 0.0 0.0))
        (if (<= (`self.Lives`) 0)
          (`GameplayStatics.OpenLevel` "Asteroids")
          (else
            (`self.ActivateShield`)))))))

(fn `ActivateShield`
  (set `self.bShielded` true)
  (`MeshComponent.SetOverlayMaterial` (`self.Ship`) "/Game/Asteroids/Materials/M_Shield.M_Shield")
  (`KismetSystemLibrary.K2_SetTimer` null "DeactivateShield" (`self.ShieldTimer`)))

(fn `AddPoints`
  (params (PointsAdded :type Integer))
  (set `self.Points` (+ PointsAdded (`self.Points`))))

(fn `DeactivateShield`
  (set `self.bShielded` false)
  (`MeshComponent.SetOverlayMaterial` (`self.Ship`) null))

(fn `EquipWeapon`
  (params (`Projectile Class` :type "/Game/Asteroids/Combat/BP_Projectile Class Reference") (Duration :type "Float (double-precision)"))
  (set `self.ActiveProjectile` `Projectile Class`)
  (`KismetSystemLibrary.K2_SetTimer` null "SetDefaultWeapon" Duration))

(fn `SetDefaultWeapon`
  (set `self.ActiveProjectile` "/Game/Asteroids/Combat/BP_LaserBlast.BP_LaserBlast_C"))

(fn `UserConstructionScript`)