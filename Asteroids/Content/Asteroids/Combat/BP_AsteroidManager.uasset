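; Asteroid wave manager for the Asteroids game that spawns the first wave on BeginPlay and a bigger one whenever the count runs out.
; Each wave activates the player's shield, then spawns asteroids and one powerup at random points sized by the Bounds box extents, centred on the world origin at fixed height.
; UpdateAsteroidCount applies a delta to the live count, incrementing the wave count and respawning at zero or below.
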(event `self.ReceiveBeginPlay`
  ;[1 1 1] Spawn the initial wave
  (`self.SpawnWave`))

(event `SpawnWave`
  (bind (_returnvalue_x _returnvalue_y) (`KismetMathLibrary.BreakVector` (`BoxComponent.GetScaledBoxExtent` (`/Game/Asteroids/General/BP_WrapBounds.Box` (`self.Bounds`)))))
  (bind _returnvalue (`KismetMathLibrary.MakeTransform` (`KismetMathLibrary.MakeVector` (`KismetMathLibrary.RandomFloatInRange` (* _returnvalue_x -1.0) _returnvalue_x) (`KismetMathLibrary.RandomFloatInRange` (* _returnvalue_y -1.0) _returnvalue_y) 70.0) (`KismetMathLibrary.RandomRotator` true) (2.0 2.0 2.0)))
  ;[1 1 1] Iterate through wave count and spawn asteroids at calculated transform
  (bind _asbp_asteroids_character (cast `/Game/Asteroids/Player/BP_AsteroidsCharacter` (`GameplayStatics.GetPlayerCharacter` 0)))
  (`/Game/Asteroids/Player/BP_AsteroidsCharacter.ActivateShield` _asbp_asteroids_character)
  (set `self.NumAsteroids` (`self.WaveCount`))
  (for _ (range (+ (`self.WaveCount`) 1))
    (`|SpawnActorFromClass` "/Game/Asteroids/Combat/BP_Asteroid.BP_Asteroid_C" _returnvalue "AlwaysSpawn" "MultiplyWithRoot" null null))
  (`|SpawnActorFromClass` "/Game/Asteroids/Combat/BP_Powerup.BP_Powerup_C" _returnvalue "Undefined" "MultiplyWithRoot" null null))

(fn `UpdateAsteroidCount`
  (params (Num :type Integer))
  ;[1 1 1] Update the asteroid count
  (set `self.NumAsteroids` (+ Num (`self.NumAsteroids`)))
  ;[1 1 1] When the count goes to zero or below, start a new wave
  (if (<= (`self.NumAsteroids`) 0)
    (`/Engine/EditorBlueprintResources/StandardMacros.IncrementInt` (`self.WaveCount`)
      (:`  `
        (`self.SpawnWave`)))))

(fn `UserConstructionScript`)