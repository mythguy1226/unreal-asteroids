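; Drifting Asteroids powerup pickup that grants the player a timed special weapon.
; On spawn it randomly picks an explosive, burst or ricochet round and sets the sphere's material to match.
; It moves each tick along a random direction flattened to the XY plane and self-destructs when its lifetime timer expires.
; Overlap with BP_AsteroidsCharacter equips that projectile class for the set duration and destroys the pickup.
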(event `self.ReceiveBeginPlay`
  (`KismetSystemLibrary.K2_SetTimer` null "SelfDestruct" (`self.Lifetime`))
  (bind _output_get (set `self.MovementDir` (`KismetMathLibrary.RandomUnitVector`)))
  (set `self.MovementDir` (`KismetMathLibrary.MakeVector` (.x _output_get) (.y _output_get)))
  (switch `int` (`KismetMathLibrary.RandomIntegerInRange` 0 2)
    (:`Default`
      (`PrimitiveComponent.SetMaterial` (`self.Sphere`) 0 "/Game/Asteroids/Materials/M_Powerup_ExplosiveRound.M_Powerup_ExplosiveRound" :!label _label)
      (set `self.AttachedWeapon` "/Game/Asteroids/Combat/BP_ExplosiveRound.BP_ExplosiveRound_C"))
    (:`0`
      (goto _label))
    (:`1`
      (`PrimitiveComponent.SetMaterial` (`self.Sphere`) 0 "/Game/Asteroids/Materials/M_Powerup_BurstRound.M_Powerup_BurstRound")
      (set `self.AttachedWeapon` "/Game/Asteroids/Combat/BP_BurstRound.BP_BurstRound_C"))
    (:`2`
      (`PrimitiveComponent.SetMaterial` (`self.Sphere`) 0 "/Game/Asteroids/Materials/M_Powerup_Ricochet.M_Powerup_Ricochet")
      (set `self.AttachedWeapon` "/Game/Asteroids/Combat/BP_RicochetRound.BP_RicochetRound_C"))))

(event `self.ReceiveTick`
  (params (DeltaSeconds :type "Float (single-precision)"))
  (`self.K2_SetActorLocation` (+ (`self.K2_GetActorLocation`) (* (`self.MovementDir`) (* DeltaSeconds (`self.Speed`))))))

(event `self.Sphere1.OnComponentBeginOverlap`
  (params (OverlappedComponent :type "PrimitiveComponent Object Reference") (OtherActor :type "Actor Object Reference") (OtherComp :type "PrimitiveComponent Object Reference") (OtherBodyIndex :type Integer) (bFromSweep :type Boolean) (SweepResult :type "HitResult Structure (by ref)"))
  (bind _asbp_asteroids_character (cast `/Game/Asteroids/Player/BP_AsteroidsCharacter` OtherActor))
  (`/Game/Asteroids/Player/BP_AsteroidsCharacter.EquipWeapon` _asbp_asteroids_character (`self.AttachedWeapon`) (`self.Duration`))
  (`self.K2_DestroyActor`))

(fn `SelfDestruct`
  (`self.K2_DestroyActor`))

(fn `UserConstructionScript`)