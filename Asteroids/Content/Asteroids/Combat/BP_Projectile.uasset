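; Asteroids projectile that flies at a set speed and splits any asteroid it hits.
; On BeginPlay it applies Speed to its ProjectileMovement component and starts a timer that calls SelfDestruct after Lifetime.
; A capsule overlap with a BP_Asteroid calls that asteroid's Split, then disables the projectile's collision and destroys it.
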(event `self.ReceiveBeginPlay`
  (bind _projectilemovement (`self.ProjectileMovement`))
  ;[1 1 1] Set the lifetime and speeds of the projectile
  (`KismetSystemLibrary.K2_SetTimer` null "SelfDestruct" (`self.Lifetime`))
  (bind _output_get (set `ProjectileMovementComponent.InitialSpeed` (`self.Speed`) _projectilemovement))
  (set `ProjectileMovementComponent.MaxSpeed` _output_get _projectilemovement))

(event `self.Capsule.OnComponentBeginOverlap`
  (params (OverlappedComponent :type "PrimitiveComponent Object Reference") (OtherActor :type "Actor Object Reference") (OtherComp :type "PrimitiveComponent Object Reference") (OtherBodyIndex :type Integer) (bFromSweep :type Boolean) (SweepResult :type "HitResult Structure (by ref)"))
  ;[1 1 1] When colliding with an asteroid, split the asteroid, disabled projectile collisions, and destroy the projectile
  (bind _asbp_asteroid (cast `/Game/Asteroids/Combat/BP_Asteroid` OtherActor))
  (`/Game/Asteroids/Combat/BP_Asteroid.Split` _asbp_asteroid)
  (`self.SetActorEnableCollision` false)
  (`self.K2_DestroyActor`))

(fn `SelfDestruct`
  ;[1 1 1] Self destruct to be called by timers
  (`self.K2_DestroyActor`))

(fn `UserConstructionScript`)