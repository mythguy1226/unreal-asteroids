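; BP_ExplosiveRound is an explosive round for the Asteroids game that splits asteroids within its blast radius.
; BeginPlay runs the parent logic, then sets the impact effect to an explosive Niagara system.
; A capsule overlap triggers a short delay, then a multi-sphere trace at the round's location calls Split on each valid BP_Asteroid hit.
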(event `self.ReceiveBeginPlay`
  (`parent.ReceiveBeginPlay`)
  (set `self.ImpactVFX` "/Game/Asteroids/VFX/Impact/NS_ExplosiveImpact.NS_ExplosiveImpact"))

(event `self.Capsule.OnComponentBeginOverlap`
  (params (OverlappedComponent :type "PrimitiveComponent Object Reference") (OtherActor :type "Actor Object Reference") (OtherComp :type "PrimitiveComponent Object Reference") (OtherBodyIndex :type Integer) (bFromSweep :type Boolean) (SweepResult :type "HitResult Structure (by ref)"))
  (bind _returnvalue (`self.K2_GetActorLocation`))
  (`KismetSystemLibrary.Delay` 0.2)
  (bind _outhits (`KismetSystemLibrary.SphereTraceMulti` _returnvalue _returnvalue (`self.BlastRadius`) "TraceTypeQuery1"))
  (for _array_element _outhits
    (bind (_bblockinghit _binitialoverlap _time _distance _location _impactpoint _normal _impactnormal _physmat _hitactor) (`GameplayStatics.BreakHitResult` _array_element))
    (`/Engine/EditorBlueprintResources/StandardMacros.IsValid` _hitactor
      (:`Is Valid`
        (bind _asbp_asteroid (cast `/Game/Asteroids/Combat/BP_Asteroid` _hitactor))
        (`/Game/Asteroids/Combat/BP_Asteroid.Split` _asbp_asteroid)))))

(fn `UserConstructionScript`
  (`parent.UserConstructionScript`))