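; BP_Asteroid is an Asteroids-style rock that drifts and splits into smaller, faster pieces.
; It picks a random XY direction on spawn, moves unswept each tick, and reverses both directions on overlapping another asteroid.
; Split awards player points by split level, updates BP_AsteroidManager's count, and spawns two half-scale children until the last level is simply destroyed.
; Children get yaw-offset rotations but choose their own random heading, and undersized ones self-destroy on BeginPlay.
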(event `self.ReceiveBeginPlay`
  (bind _returnvalue_x (`KismetMathLibrary.BreakVector` (`self.GetActorScale3D`)))
  ;[1 1 1] On spawning, start moving in a random direction
  (bind _output_get (set `self.MovementDir` (`KismetMathLibrary.RandomUnitVector`)))
  (set `self.MovementDir` (`KismetMathLibrary.MakeVector` (.x _output_get) (.y _output_get)))
  (if (< _returnvalue_x 0.125)
    (`self.K2_DestroyActor`)))

(event `self.ReceiveTick`
  (params (DeltaSeconds :type "Float (single-precision)"))
  ;[1 1 1] Calculate new position for the asteroid for movement
  (`self.K2_SetActorLocation` (+ (`self.K2_GetActorLocation`) (* (`self.MovementDir`) (* DeltaSeconds (`self.Speed`))))))

(event `self.Capsule.OnComponentBeginOverlap`
  (params (OverlappedComponent :type "PrimitiveComponent Object Reference") (OtherActor :type "Actor Object Reference") (OtherComp :type "PrimitiveComponent Object Reference") (OtherBodyIndex :type Integer) (bFromSweep :type Boolean) (SweepResult :type "HitResult Structure (by ref)"))
  (bind _asbp_asteroid (cast `/Game/Asteroids/Combat/BP_Asteroid` OtherActor))
  (set `/Game/Asteroids/Combat/BP_Asteroid.MovementDir` (* (`/Game/Asteroids/Combat/BP_Asteroid.MovementDir` _asbp_asteroid) -1.0) _asbp_asteroid)
  (set `self.MovementDir` (* (`self.MovementDir`) -1.0)))

(fn `Split`
  (bind _asbp_asteroids_character (cast `/Game/Asteroids/Player/BP_AsteroidsCharacter` (`GameplayStatics.GetPlayerCharacter` 0)))
  (switch `int` (`self.SplitLevel`)
    (:`0`
      (`/Game/Asteroids/Player/BP_AsteroidsCharacter.AddPoints` _asbp_asteroids_character 20))
    (:`1`
      (`/Game/Asteroids/Player/BP_AsteroidsCharacter.AddPoints` _asbp_asteroids_character 50))
    (:`2`
      (`/Game/Asteroids/Player/BP_AsteroidsCharacter.AddPoints` _asbp_asteroids_character 100)))
  (bind _returnvalue (`GameplayStatics.GetActorOfClass` "/Game/Asteroids/Combat/BP_AsteroidManager.BP_AsteroidManager_C"))
  (if (> (`self.SplitLevel`) 1)
    (`/Game/Asteroids/Combat/BP_AsteroidManager.UpdateAsteroidCount` _returnvalue -1)
    (`self.K2_DestroyActor`)
    (else
      (`/Game/Asteroids/Combat/BP_AsteroidManager.UpdateAsteroidCount` _returnvalue 1)
      (bind _returnvalue_2 (`|SpawnActorFromClass` "BP_Asteroid_C" (`KismetMathLibrary.MakeTransform` (`self.K2_GetActorLocation`) (`KismetMathLibrary.Quat_Rotator` (* (`KismetMathLibrary.Conv_RotatorToQuaternion` (`self.K2_GetActorRotation`)) (`KismetMathLibrary.Conv_RotatorToQuaternion` (`KismetMathLibrary.RotatorFromAxisAndAngle` (0.0 0.0 1.0) 30.0)))) (* (`self.GetActorScale3D`) 0.5)) "AlwaysSpawn" "MultiplyWithRoot" null null))
      (`/Engine/EditorBlueprintResources/StandardMacros.IsValid` _returnvalue_2
        (:`Is Valid`
          (set `/Game/Asteroids/Combat/BP_Asteroid.SplitLevel` (+ (`self.SplitLevel`) 1) _returnvalue_2)
          (set `/Game/Asteroids/Combat/BP_Asteroid.Speed` (* (`self.Speed`) 1.1) _returnvalue_2)
          (bind _returnvalue_3 (`|SpawnActorFromClass` "BP_Asteroid_C" (`KismetMathLibrary.MakeTransform` (`self.K2_GetActorLocation`) (`KismetMathLibrary.Quat_Rotator` (* (`KismetMathLibrary.Conv_RotatorToQuaternion` (`self.K2_GetActorRotation`)) (`KismetMathLibrary.Conv_RotatorToQuaternion` (`KismetMathLibrary.RotatorFromAxisAndAngle` (0.0 0.0 1.0) -30.0)))) (* (`self.GetActorScale3D`) 0.5)) "AlwaysSpawn" "MultiplyWithRoot" null null))
          (`/Engine/EditorBlueprintResources/StandardMacros.IsValid` _returnvalue_3
            (:`Is Valid`
              (set `/Game/Asteroids/Combat/BP_Asteroid.SplitLevel` (+ (`self.SplitLevel`) 1) _returnvalue_3)
              (set `/Game/Asteroids/Combat/BP_Asteroid.Speed` (* (`self.Speed`) 1.1) _returnvalue_3)
              (`self.K2_DestroyActor`))))))))

(fn `UserConstructionScript`)