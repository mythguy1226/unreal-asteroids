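; Screen-wrap boundary for the Asteroids game that moves actors leaving its Box to the opposite edge.
; The Box's end-overlap event passes the exiting actor to WrapTopDown for the X axis and WrapLeftRight for the Y axis, keeping Z unchanged.
; Both compare world location against plus or minus the scaled box extent, so the math assumes the Box is centered on the world origin.
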(event `self.Box.OnComponentEndOverlap`
  (params (OverlappedComponent :type "PrimitiveComponent Object Reference") (OtherActor :type "Actor Object Reference") (OtherComp :type "PrimitiveComponent Object Reference") (OtherBodyIndex :type Integer))
  ;[1 1 1] If an actor is leaving the bounds then detect sides to wrap to
  (`self.WrapTopDown` OtherActor)
  (`self.WrapLeftRight` OtherActor))

(fn `UserConstructionScript`)

(fn `WrapLeftRight`
  (params (Actor :type "Actor Object Reference"))
  (locals (MovingActor :type "Actor Object Reference"))
  (bind (_returnvalue_x _returnvalue_y _returnvalue_z) (`KismetMathLibrary.BreakVector` (`self.K2_GetActorLocation` (`local.MovingActor`))))
  (bind (_returnvalue_x_2 _returnvalue_y_2) (`KismetMathLibrary.BreakVector` (`BoxComponent.GetScaledBoxExtent` (`self.Box`))))
  (bind (_returnvalue_x_3 _returnvalue_y_3 _returnvalue_z_2) (`KismetMathLibrary.BreakVector` (`self.K2_GetActorLocation` (`local.MovingActor`))))
  (bind (_returnvalue_x_4 _returnvalue_y_4) (`KismetMathLibrary.BreakVector` (`BoxComponent.GetScaledBoxExtent` (`self.Box`))))
  ;[1 1 1] Check if the right side has been reached; if so set the actor to the left side
  (set `local.MovingActor` Actor)
  (if (> _returnvalue_y _returnvalue_y_2)
    (`self.K2_SetActorLocation` (`local.MovingActor`) (`KismetMathLibrary.MakeVector` _returnvalue_x (* _returnvalue_y_2 -1.0) _returnvalue_z) false false)
    (else
      ;[1 1 1] Check if the left side has been reached; if so set actor to the right side
      (if (< _returnvalue_y_3 (* _returnvalue_y_4 -1.0))
        (`self.K2_SetActorLocation` (`local.MovingActor`) (`KismetMathLibrary.MakeVector` _returnvalue_x_3 _returnvalue_y_4 _returnvalue_z_2) false false)))))

(fn `WrapTopDown`
  (params (Actor :type "Actor Object Reference"))
  (locals (MovingActor :type "Actor Object Reference"))
  (bind (_returnvalue_x _returnvalue_y _returnvalue_z) (`KismetMathLibrary.BreakVector` (`self.K2_GetActorLocation` (`local.MovingActor`))))
  (bind _returnvalue_x_2 (`KismetMathLibrary.BreakVector` (`BoxComponent.GetScaledBoxExtent` (`self.Box`))))
  (bind (_returnvalue_x_3 _returnvalue_y_2 _returnvalue_z_2) (`KismetMathLibrary.BreakVector` (`self.K2_GetActorLocation` (`local.MovingActor`))))
  (bind _returnvalue_x_4 (`KismetMathLibrary.BreakVector` (`BoxComponent.GetScaledBoxExtent` (`self.Box`))))
  ;[1 1 1] Check if the top side has been reached; if so set the actor to the bottom side
  (set `local.MovingActor` Actor)
  (if (> _returnvalue_x _returnvalue_x_2)
    (`self.K2_SetActorLocation` (`local.MovingActor`) (`KismetMathLibrary.MakeVector` (* _returnvalue_x_2 -1.0) _returnvalue_y _returnvalue_z) false false)
    (else
      ;[1 1 1] Check if the bottom side has been reached; if so set actor to the top side
      (if (< _returnvalue_x_3 (* _returnvalue_x_4 -1.0))
        (`self.K2_SetActorLocation` (`local.MovingActor`) (`KismetMathLibrary.MakeVector` _returnvalue_x_4 _returnvalue_y_2 _returnvalue_z_2) false false)))))